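; BP_BaseProjectile is a projectile actor that handles firing and impact feedback.
; On BeginPlay it plays the shot sound, then sets an Armed flag after a very short delay, so earlier overlaps are ignored.
; Once armed, a Sphere overlap spawns the OnHit effect with negated actor rotation, calls an impact sound and destroys the actor.
; The graph applies no damage.
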(event `self.ReceiveBeginPlay`
  (`GameplayStatics.PlaySoundAtLocation` "/Game/STARTHERE/FX/Projectiles/Shot.Shot" (`self.K2_GetActorLocation`) (struct) 0.65 1.0 0.0 null null null null)
  (`KismetSystemLibrary.Delay` 0.02)
  (set `self.Armed` true))

(event `self.Sphere.OnComponentBeginOverlap`
  (params (OverlappedComponent :type "PrimitiveComponent Object Reference") (OtherActor :type "Actor Object Reference") (OtherComp :type "PrimitiveComponent Object Reference") (OtherBodyIndex :type Integer) (bFromSweep :type Boolean) (SweepResult :type "HitResult Structure (by ref)"))
  (bind _returnvalue (`self.K2_GetActorLocation`))
  (if (`self.Armed`)
    (`NiagaraFunctionLibrary.SpawnSystemAtLocation` (`self.OnHit`) _returnvalue (* (`self.K2_GetActorRotation`) -1.0))
    (`GameplayStatics.PlaySoundAtLocation` null _returnvalue (struct) 1.0 1.0 0.0 null null null null)
    (`self.K2_DestroyActor`)))

(fn `UserConstructionScript`)