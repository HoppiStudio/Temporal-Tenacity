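; Base cover actor for a game with past and present states, setting health, destructibility, box extent and world cover points from its cover type and settings at construction.
; Overlapping actors receive the cover type, and the TemporalTelemetryManager is told when enemies or players leave.
; Damage to destructible cover notifies its LinkedCover: a past-side call destroys that cover and reports to the manager, otherwise it only clears its link.
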(event `self.ReceiveBeginPlay`
  (`KismetSystemLibrary.Delay` 0.2)
  (`self.Init`))

(event `Init`
  (bind _outactors (`GameplayStatics.GetAllActorsOfClass` "/Game/STARTHERE/Blueprints/Gamemodes/GameRules/TemporalTelemetryManager.TemporalTelemetryManager_C"))
  (for _array_element _outactors
    (set `self.TTManager` _array_element)))

(event `self.ReceiveActorBeginOverlap`
  (params (OtherActor :type "Actor Object Reference"))
  (message `/Game/STARTHERE/Library/Interfaces/CombatInterface.ChangeCoverType` OtherActor (`self.Cover Type`)))

(event `self.ReceiveAnyDamage`
  (params (Damage :type "Float (single-precision)") (DamageType :type "DamageType Object Reference") (InstigatedBy :type "Controller Object Reference") (DamageCauser :type "Actor Object Reference"))
  (bind _linkedcover (`self.LinkedCover`))
  ;[1 1 1] Damage & Health
  (if (`self.Destructable`)
    (bind _output_get (set `self.HP` (- (`self.HP`) Damage)))
    (if (and (<= _output_get 0.0) (`self.Past`))
      (`/Engine/EditorBlueprintResources/StandardMacros.IsValid` _linkedcover
        (:`Is Valid`
          (`/Game/STARTHERE/Library/Interfaces/CombatInterface.CoverDestroyed` _linkedcover true))
        (:`Is Not Valid`
          _))
      (else
        (`/Game/STARTHERE/Library/Interfaces/CombatInterface.CoverDestroyed` _linkedcover false)))
    (`KismetSystemLibrary.Delay` 0.5)
    (`self.K2_DestroyActor`)))

(event `/Game/STARTHERE/Library/Interfaces/CombatInterface.CoverDestroyed`
  (params (Past :type Boolean))
  ;[1 1 1] TemporalTelem
  (if Past
    (message `/Game/STARTHERE/Library/Interfaces/TTInterface.TTEventCoverDestroyed` (`self.TTManager`) self)
    (`KismetSystemLibrary.Delay` 0.5)
    (`self.K2_DestroyActor`)
    (else
      (set `self.LinkedCover` null))))

(event `self.ReceiveActorEndOverlap`
  (params (OtherActor :type "Actor Object Reference"))
  (bind _ttmanager (`self.TTManager`))
  ;[1 1 1] TemporalTelem
  (bind _asbp_base_enemy (cast `/Game/STARTHERE/Blueprints/Enemies/BP_BaseEnemy` OtherActor)
    (:`then`
      (message `/Game/STARTHERE/Library/Interfaces/TTInterface.EnemyLeaveCover` _ttmanager _asbp_base_enemy self))
    (:`CastFailed`
      (bind _asbp_base_character (cast `/Game/STARTHERE/Blueprints/Character/BP_BaseCharacter` OtherActor))
      (message `/Game/STARTHERE/Library/Interfaces/TTInterface.PlayerLeaveCover` _ttmanager _asbp_base_character self))))

(fn `CheckCover`
  (returns (Cover :type "/Game/STARTHERE/Library/Enums/CoverEnum Enum"))
  (return "NewEnumerator0"))

(fn `GetTargetLoc`
  (returns (Loc :type "Vector Structure"))
  (return (0.0 0.0 0.0)))

(fn `Identify`
  (returns (Idenity :type "/Game/STARTHERE/Library/Enums/IdentifyEnum Enum") (Ref :type "Actor Object Reference"))
  (return "NewEnumerator0" null))

(fn `UserConstructionScript`
  (bind _cover_type (`self.Cover Type`))
  (set `self.HP` (select `/Game/STARTHERE/Library/Enums/CoverEnum` _cover_type :`NewEnumerator0` 1.0 :`NewEnumerator1` 1.0 :`NewEnumerator2` 8.0 :`NewEnumerator3` 20.0 :`NewEnumerator4` 40.0))
  (set `self.Destructable` (select `/Game/STARTHERE/Library/Enums/CoverEnum` _cover_type :`NewEnumerator2` true :`NewEnumerator3` true :`NewEnumerator4` true))
  (`BoxComponent.SetBoxExtent` (`self.Box`) (`self.BoxExtent`) true)
  (for (_array_element _array_index) (`self.CoverPoints`)
    (`KismetArrayLibrary.Array_Set` (`self.CoverLocs`) _array_index (+ (`self.K2_GetActorLocation`) _array_element))))