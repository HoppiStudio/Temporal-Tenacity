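; BP_Base_interaction is a base interaction Blueprint with a collision component and an E key prompt flow, largely left as stubs.
; Begin overlap and the E press, gated on Interacting, take no action.
; End overlap clears the stored character and flag and hides the Collect_bp widget.
; The logic that detects BP_BaseCharacter and creates that widget for player 0 is disconnected, marked for multiplayer rework.
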(event `self.CollisionComponent.OnComponentBeginOverlap`
  (params (OverlappedComponent :type "PrimitiveComponent Object Reference") (OtherActor :type "Actor Object Reference") (OtherComp :type "PrimitiveComponent Object Reference") (OtherBodyIndex :type Integer) (bFromSweep :type Boolean) (SweepResult :type "HitResult Structure (by ref)")))

(event `Key|E`
  (params (Key :type "Key Structure"))
  (:`Pressed`
    (if (`self.Interacting`)
      _)))

(event `self.CollisionComponent.OnComponentEndOverlap`
  (params (OverlappedComponent :type "PrimitiveComponent Object Reference") (OtherActor :type "Actor Object Reference") (OtherComp :type "PrimitiveComponent Object Reference") (OtherBodyIndex :type Integer))
  (if (== OtherActor (`self.Char Ref`))
    (set `self.Char Ref` null)
    (set `self.Interacting` false)
    (`Widget.SetVisibility` (`self.Colect Txt`) "Hidden")))

(fn `UserConstructionScript`)