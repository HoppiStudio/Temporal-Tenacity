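; EnemiesRemainingWinTrigger is a win condition that opens a target level once the enemy count drops to a set threshold.
; On BeginPlay it finds all enemy actors in the level and binds to their EnemyDead events.
; Each death triggers a half-second delay and a fresh count, which either opens the level or prints the number of enemies remaining.
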(event `self.ReceiveBeginPlay`
  ;[1 1 1] On Play, Get All Enemies In The Level and Subscribe To Their Death Events
  (bind _outactors (`GameplayStatics.GetAllActorsOfClass` "/Game/STARTHERE/Blueprints/Enemies/Target.Target_C"))
  (add `/Game/STARTHERE/Blueprints/Enemies/BP_BaseEnemy.EnemyDead` _outactors (delegate `OnEnemyDeath`)))

(event `OnEnemyDeath`
  ;[1 1 1] Check How Many Enemies Remain In The Level Whenever The Enemy Dead Event Is Invoked. Load Next Level If No More Enemies Remain
  (`KismetSystemLibrary.Delay` 0.5)
  (bind _outactors (`GameplayStatics.GetAllActorsOfClass` "/Game/STARTHERE/Blueprints/Enemies/Target.Target_C"))
  (bind _returnvalue (`KismetArrayLibrary.Array_Length` _outactors))
  (if (<= _returnvalue (`self.EnemiesRemainingToWin`))
    (`GameplayStatics.OpenLevelBySoftObjectPtr` (`self.Level`))
    (else
      (`KismetSystemLibrary.PrintString` (`KismetStringLibrary.Concat_StrStr` "Enemies Remaining: " (`KismetStringLibrary.Conv_IntToString` _returnvalue))))))

(fn `UserConstructionScript`)