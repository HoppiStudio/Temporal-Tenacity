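; Base enemy Blueprint that tracks health, updates its health bar and handles its own death.
; BeginPlay stores starting health as the maximum, and damage and state events push health and state index to the widget through EnemyInfoMessage.
; At zero health it calls EnemyDead, spawns a bloody explosion and destroys itself after a short delay.
; Query functions expose identity, index and cover, while player, time-zone and pause functions are default-returning stubs.
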(event `self.ReceiveBeginPlay`
  ;[1 1 1] Init
  (`self.Init`))

(event `Init`
  (bind _health (`self.Health`))
  ;[1 1 1] Init
  (bind _output_get (set `self.MaxHealth` _health))
  (message `/Game/STARTHERE/Library/Interfaces/UIInterface.EnemyInfo` (`WidgetComponent.GetWidget` (`self.Healthbar`)) _health _output_get 0))

(event `self.ReceiveAnyDamage`
  (params (Damage :type "Float (single-precision)") (DamageType :type "DamageType Object Reference") (InstigatedBy :type "Controller Object Reference") (DamageCauser :type "Actor Object Reference"))
  ;[0 0.2202 1] TEMPORAL TELEMETRY NEEDED
  (bind _output_get (set `self.Health` (- (`self.Health`) Damage)))
  (message `/Game/STARTHERE/Library/Interfaces/UIInterface.EnemyInfo` (`WidgetComponent.GetWidget` (`self.Healthbar`)) _output_get (`self.MaxHealth`) (`self.StateIndex`))
  (if (<= _output_get 0.0)
    (`self.EnemyDead`)
    (`NiagaraFunctionLibrary.SpawnSystemAtLocation` "/Game/STARTHERE/FX/ParticleEffects/BloodyExplosion.BloodyExplosion" (`self.K2_GetActorLocation`))
    (`KismetSystemLibrary.Delay` 0.2)
    (`self.K2_DestroyActor`)))

(event `/Game/STARTHERE/Library/Interfaces/GMInterface.AssignEnemyIndex`
  (params (Index :type Integer))
  ;[0 0.2202 1] TEMPORAL TELEMETRY NEEDED
  (set `self.Index` Index))

(event `/Game/STARTHERE/Library/Interfaces/UIInterface.EnemyInfo`
  (params (HP :type "Float (double-precision)") (MaxHP :type "Float (double-precision)") (StateIndex :type Integer))
  (bind _output_get (set `self.Index` StateIndex))
  (message `/Game/STARTHERE/Library/Interfaces/UIInterface.EnemyInfo` (`WidgetComponent.GetWidget` (`self.Healthbar`)) (`self.Health`) (`self.MaxHealth`) _output_get))

(fn `CanDestroyCover`
  (returns (`True?` :type Boolean))
  (return false))

(fn `CheckCover`
  (returns (Cover :type "/Game/STARTHERE/Library/Enums/CoverEnum Enum"))
  (return (`self.Cover`)))

(fn `GetEnemyIndex`
  (returns (Index :type Integer))
  (return (`self.Index`)))

(fn `GetPlayerIndex`
  (returns (PlayerIndex :type Integer))
  (return 0))

(fn `GetPlayers`
  (returns (Actors :type "Array of Actor Object Reference") (Success :type Boolean))
  (return _ false))

(fn `GetTargetLoc`
  (returns (Loc :type "Vector Structure"))
  (return (0.0 0.0 0.0)))

(fn `GetTimeZone`
  (returns (`Past?` :type Boolean))
  (return false))

(fn `Identify`
  (returns (Idenity :type "/Game/STARTHERE/Library/Enums/IdentifyEnum Enum") (Ref :type "Actor Object Reference"))
  (return (`self.Identity`) self))

(fn `InPast?`
  (returns (`Past?` :type Boolean))
  (return false))

(fn `PauseEnemies`
  (params (Pause :type Boolean) (UnPauseData :type "/Game/STARTHERE/Library/Structs/PauseEnemy Structure"))
  (returns (PauseData :type "/Game/STARTHERE/Library/Structs/PauseEnemy Structure"))
  (return))

(fn `PauseGame`
  (params (Pause :type Boolean) (UnPauseData :type "/Game/STARTHERE/Library/Structs/PauseGame Structure"))
  (returns (PauseData :type "/Game/STARTHERE/Library/Structs/PauseGame Structure"))
  (return))

(fn `PausePlayers`
  (params (Pause :type Boolean) (UnPauseData :type "/Game/STARTHERE/Library/Structs/PausePlayer Structure"))
  (returns (Pausedata :type "/Game/STARTHERE/Library/Structs/PausePlayer Structure"))
  (return))

(fn `PlayerHealth`
  (params (Index :type Integer))
  (returns (HP :type "Float (double-precision)") (Success :type Boolean))
  (return 0.0 false))

(fn `SelectedPlayer`
  (returns (PlayerIndex :type Integer))
  (return 0))

(fn `UserConstructionScript`)