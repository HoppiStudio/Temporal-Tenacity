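; Enemy spawner that populates a navigable area while a player character is inside its trigger sphere.
; Overlap starts a spawn immediately and on a timer, placing pawns at random navmesh points with an FX burst until its tracked list reaches the cap.
; Each spawn receives an index message from the game mode and is announced via EnemySpawned.
; Exit stops the timer and, after a delay, destroys surviving spawns with FX.
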(event `SpawnEnemy`
  ;[1 1 1] Spawn Enemy If The EnemySpawner Population Is Below The Max Spawn Count Threshold
  (if (< (`KismetArrayLibrary.Array_Length` (`self.Enemies`)) (`self.MaxEnemies`))
    ;[1 1 1] Set The Spawn Position To a Random (Navigable) Point Within The Radius of The Enemy Spawner Location Point
    (bind _output_get (set `self.EnemySpawnLocation` (`SceneComponent.K2_GetComponentLocation` (`self.EnemySpawnLocationSphere`))))
    (bind _randomlocation (`NavigationSystemV1.K2_GetRandomLocationInNavigableRadius` _output_get (`SphereComponent.SphereRadius` (`self.Sphere`)) null null))
    ;[1 1 1] FX
    (`NiagaraFunctionLibrary.SpawnSystemAtLocation` "/Game/STARTHERE/FX/ParticleEffects/RechieveDamageWithTemporalTanacity.RechieveDamageWithTemporalTanacity" _randomlocation)
    ;[1 1 1] Spawn An Enemy and Add It To The List of Spawned Enemies (for THIS spawner)
    (bind _returnvalue (`|SpawnActorFromClass` (`self.Pawn Class`) (`KismetMathLibrary.Conv_VectorToTransform` _randomlocation) (`self.Collision Handling Override`) "OverrideRootScale" null null))
    (`KismetArrayLibrary.Array_Add` (`self.Enemies`) _returnvalue)
    (bind _index (message `/Game/STARTHERE/Library/Interfaces/GMInterface.GetEnemyIndex` (`GameplayStatics.GetGameMode`)))
    (`/Engine/EditorBlueprintResources/StandardMacros.IsValid` _returnvalue
      (:`Is Valid`
        (message `/Game/STARTHERE/Library/Interfaces/GMInterface.AssignEnemyIndex` _returnvalue _index)
        (bind _asbp_base_enemy (cast `/Game/STARTHERE/Blueprints/Enemies/BP_BaseEnemy` _returnvalue))
        (`self.EnemySpawned` _asbp_base_enemy)))))

(event `self.Sphere.OnComponentBeginOverlap`
  (params (OverlappedComponent :type "PrimitiveComponent Object Reference") (OtherActor :type "Actor Object Reference") (OtherComp :type "PrimitiveComponent Object Reference") (OtherBodyIndex :type Integer) (bFromSweep :type Boolean) (SweepResult :type "HitResult Structure (by ref)"))
  ;[1 1 1] If Player Enters Spawner Bounds Invoke The SpawnEnemy Callback and Initiate The Timer For Spawning Enemies
  (cast `/Game/STARTHERE/Blueprints/Character/BP_BaseCharacter` OtherActor)
  (`self.SpawnEnemy`)
  (bind _returnvalue (`KismetSystemLibrary.K2_SetTimerDelegate` (delegate `SpawnEnemy`) (`KismetMathLibrary.Conv_IntToDouble` (`self.SpawnRate`)) (`self.Loop`)))
  (set `self.SpawnTimer` _returnvalue))

(event `self.Sphere.OnComponentEndOverlap`
  (params (OverlappedComponent :type "PrimitiveComponent Object Reference") (OtherActor :type "Actor Object Reference") (OtherComp :type "PrimitiveComponent Object Reference") (OtherBodyIndex :type Integer))
  (bind _enemies (`self.Enemies`))
  ;[1 1 1] Stop Timer When Player Has Exited Spawner Bounds
  (cast `/Game/STARTHERE/Blueprints/Character/BP_BaseCharacter` OtherActor)
  (`KismetSystemLibrary.K2_ClearAndInvalidateTimerHandle` (`self.SpawnTimer`))
  ;[1 1 1] After Exiting Spawner Bounds, Destroy Any Spawned Enemies (From This Spawner) If They Still Exist
  (`KismetSystemLibrary.Delay` (`self.DespawnDelay`))
  (for _array_element _enemies
    (if (`KismetSystemLibrary.IsValid` _array_element)
      (`NiagaraFunctionLibrary.SpawnSystemAtLocation` "/Game/STARTHERE/FX/ParticleEffects/RechieveDamageWithTemporalTanacity.RechieveDamageWithTemporalTanacity" (`self.K2_GetActorLocation` _array_element))
      (`self.K2_DestroyActor` _array_element)))
  (`KismetArrayLibrary.Array_Clear` _enemies))

(fn `GetEnemyIndex`
  (returns (Index :type Integer))
  (return 0))

(fn `GetPlayerIndex`
  (returns (PlayerIndex :type Integer))
  (return 0))

(fn `GetPlayers`
  (returns (Actors :type "Array of Actor Object Reference") (Success :type Boolean))
  (return _ false))

(fn `InPast?`
  (returns (`Past?` :type Boolean))
  (return false))

(fn `PauseEnemies`
  (params (Pause :type Boolean) (UnPauseData :type "/Game/STARTHERE/Library/Structs/PauseEnemy Structure"))
  (returns (PauseData :type "/Game/STARTHERE/Library/Structs/PauseEnemy Structure"))
  (return))

(fn `PauseGame`
  (params (Pause :type Boolean) (UnPauseData :type "/Game/STARTHERE/Library/Structs/PauseGame Structure"))
  (returns (PauseData :type "/Game/STARTHERE/Library/Structs/PauseGame Structure"))
  (return))

(fn `PausePlayers`
  (params (Pause :type Boolean) (UnPauseData :type "/Game/STARTHERE/Library/Structs/PausePlayer Structure"))
  (returns (Pausedata :type "/Game/STARTHERE/Library/Structs/PausePlayer Structure"))
  (return))

(fn `UserConstructionScript`)