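; Enemy turret that repeatedly damages BP_BaseCharacter actors within TurretRange.
; After a short BeginPlay delay it caches all characters, then a looping timer checks their distances, keeping the last one in range as target.
; A self-rearming one-shot timer applies damage, its delay derived from the target's CheckCover result through per-cover values in Timers0.
; The timer is cleared when nobody is in range.
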(event `self.ReceiveBeginPlay`
  (`parent.ReceiveBeginPlay`)
  (`KismetSystemLibrary.Delay` 1.0)
  (bind _outactors (`GameplayStatics.GetAllActorsOfClass` "/Game/STARTHERE/Blueprints/Character/BP_BaseCharacter.BP_BaseCharacter_C"))
  (set `self.Characters` _outactors)
  (`KismetSystemLibrary.K2_SetTimerDelegate` (delegate `TurretSight`) 0.5 true))

(event `TurretSight`
  (bind (_timers_0_disadvantage _timers_0_open _timers_0_light _timers_0_medium _timers_0_heavy _timers_0_full) (break `/Game/STARTHERE/Library/Structs/DamageTimers` (`self.Timers_0`)))
  (for _array_element (`self.Characters`)
    (if (<= (`self.GetDistanceTo` _array_element self) (`self.TurretRange`))
      (set `self.TargetChar` _array_element)
      (set `self.Alert` true)))
  (if (`self.Alert`)
    (set `self.Alert` false)
    (if (not (`self.Shooting`))
      (set `self.Shooting` true)
      (bind _cover (`/Game/STARTHERE/Library/Interfaces/CombatInterface.CheckCover` (`self.TargetChar`) :!label _label))
      (bind _returnvalue (select `/Game/STARTHERE/Library/Enums/CoverEnum` _cover :`NewEnumerator0` _timers_0_disadvantage :`NewEnumerator1` _timers_0_open :`NewEnumerator2` _timers_0_light :`NewEnumerator3` _timers_0_medium :`NewEnumerator4` _timers_0_heavy :`NewEnumerator5` _timers_0_full :!type "Float (single-precision)"))
      (bind _returnvalue_2 (`KismetSystemLibrary.K2_SetTimerDelegate` (delegate `Shoot`) (/ _returnvalue (`KismetMathLibrary.SelectFloat` 0.1 3.0 (> _returnvalue 0.0))))))
    (else
      (`KismetSystemLibrary.K2_ClearAndInvalidateTimerHandle` _returnvalue_2)
      (set `self.Shooting` false))))

(event `Shoot`
  (bind _targetchar (`self.TargetChar`))
  (`/Engine/EditorBlueprintResources/StandardMacros.IsValid` _targetchar
    (:`Is Valid`
      (`GameplayStatics.ApplyDamage` _targetchar 1.0)
      (`KismetSystemLibrary.K2_ClearAndInvalidateTimerHandle` (stale `TurretSight` _returnvalue_2))
      (goto _label))))

(fn `UserConstructionScript`
  (`parent.UserConstructionScript`))