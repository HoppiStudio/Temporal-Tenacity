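; In-game HUD actor that creates the player's on-screen UI and the time travel screen effect.
; On BeginPlay, Init creates UI_InGame and TimeTravelEffect widgets for player 0 and adds them to the player screen, with the HUD layered above the effect.
; TimeTravelFX forwards to the effect widget's TimeTravelFXMessage.
; GetTimeZone and PlayerHealth are stubs that return only default values.
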(event `self.ReceiveBeginPlay`
  (`self.Init`))

(event `Init`
  (bind _returnvalue (`|CreateWidget` "/Game/STARTHERE/UI/UI_InGame.UI_InGame_C" (`GameplayStatics.GetPlayerController` 0)))
  (bind _output_get (set `self.Hud` _returnvalue))
  (`UserWidget.AddToPlayerScreen` _output_get 1)
  (bind _returnvalue_2 (`|CreateWidget` "/Game/STARTHERE/UI/assets/Effects/TimeTravelEffect.TimeTravelEffect_C" (`GameplayStatics.GetPlayerController` 0)))
  (set `self.TTFX` _returnvalue_2)
  (`UserWidget.AddToPlayerScreen` _returnvalue_2 0))

(event `/Game/STARTHERE/Library/Interfaces/UIInterface.TimeTravelFX`
  (message `/Game/STARTHERE/Library/Interfaces/UIInterface.TimeTravelFX` (`self.TTFX`)))

(fn `GetTimeZone`
  (returns (`Past?` :type Boolean))
  (return false))

(fn `PlayerHealth`
  (params (Index :type Integer))
  (returns (HP :type "Float (double-precision)") (Success :type Boolean))
  (return 0.0 false))

(fn `UserConstructionScript`)