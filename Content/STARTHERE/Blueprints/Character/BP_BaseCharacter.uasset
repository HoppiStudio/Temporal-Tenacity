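; Base class for AI-controlled player characters, handling health, timed combat, cover and past/present time-zone state.
; A half-second timer feeds controller state and HP to a child-actor status icon.
; BeginCombat sets timers from the target's cover: Shoot applies damage and re-checks cover, while looping tracers spawn with narrowing random spread.
; Target death clears combat timers; own death only prints and plays a sound, and most interface functions are stubs.
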(event `self.ReceiveBeginPlay`
  (`KismetSystemLibrary.Delay` 0.2)
  (`self.Init`))

(event `Init`
  (bind _asbp_character_state_object (cast `/Game/STARTHERE/Blueprints/Character/BP_CharacterStateObject` (`ChildActorComponent.ChildActor` (`self.ChildActor`)))
    (:`then`
      (set `self.StateIcon` _asbp_character_state_object)
      (`KismetSystemLibrary.K2_SetTimerDelegate` (delegate `StateSwap`) 0.5 true))
    (:`CastFailed`
      _))
  (`KismetSystemLibrary.Delay` 0.5)
  (bind _asplayer_aicontroller (cast `/Game/STARTHERE/AI/Player/PlayerAIController` (`AIBlueprintHelperLibrary.GetAIController` self)))
  (set `self.Index` (`/Game/STARTHERE/AI/Player/PlayerAIController.Index` _asplayer_aicontroller)))

(event `StateSwap`
  (bind _state (message `/Game/STARTHERE/Library/Interfaces/InputInterface.CheckState` (`AIBlueprintHelperLibrary.GetAIController` self)))
  (`/Game/STARTHERE/Blueprints/Character/BP_CharacterStateObject.UpdateInfo` (`self.StateIcon`) (`self.Index`) _state (`self.HP`)))

(event `self.ReceiveAnyDamage`
  (params (Damage :type "Float (single-precision)") (DamageType :type "DamageType Object Reference") (InstigatedBy :type "Controller Object Reference") (DamageCauser :type "Actor Object Reference"))
  ;[1 1 1] Health & Death
  (bind _output_get (set `self.HP` (- (`self.HP`) Damage)))
  (if (<= _output_get 0.0)
    (`KismetSystemLibrary.PrintString` "IM DEAD")
    (`GameplayStatics.PlaySound2D` "/Game/StarterContent/Audio/Collapse01.Collapse01" 0.2 1.0 0.0 null null)))

(event `/Game/STARTHERE/Library/Interfaces/CombatInterface.EndCombat`
  ;[1 1 1] Combat
  (bind _asbp_base_enemy (cast `/Game/STARTHERE/Blueprints/Enemies/BP_BaseEnemy` (`self.CurrentTarget`))
    (:`then`
      (clear `/Game/STARTHERE/Blueprints/Enemies/BP_BaseEnemy.EnemyDead` _asbp_base_enemy))
    (:`CastFailed`
      _))
  (`KismetSystemLibrary.K2_ClearAndInvalidateTimerHandle` (stale `/Game/STARTHERE/Library/Interfaces/CombatInterface.BeginCombat` _returnvalue_3))
  (`KismetSystemLibrary.K2_ClearAndInvalidateTimerHandle` (stale `/Game/STARTHERE/Library/Interfaces/CombatInterface.BeginCombat` _returnvalue_4)))

(event `/Game/STARTHERE/Library/Interfaces/CombatInterface.BeginCombat`
  (params (Enemy :type "Actor Object Reference"))
  (bind (_timers_disadvantage _timers_open _timers_light _timers_medium _timers_heavy _timers_full) (break `/Game/STARTHERE/Library/Structs/DamageTimers` (`self.Timers`)))
  ;[1 1 1] Combat
  (bind _output_get (set `self.CurrentTarget` Enemy))
  (bind _asbp_base_enemy (cast `/Game/STARTHERE/Blueprints/Enemies/BP_BaseEnemy` _output_get)
    (:`then`
      (add `/Game/STARTHERE/Blueprints/Enemies/BP_BaseEnemy.EnemyDead` _asbp_base_enemy (delegate `EnemyDead`)))
    (:`CastFailed`
      _))
  (bind _cover (message `/Game/STARTHERE/Library/Interfaces/CombatInterface.CheckCover` _output_get :!label _label))
  (switch `/Game/STARTHERE/Library/Enums/CoverEnum` _cover
    (:`NewEnumerator0`
      _)
    (:`NewEnumerator1`
      _)
    (:`NewEnumerator2`
      _)
    (:`NewEnumerator3`
      _)
    (:`NewEnumerator4`
      _))
  (bind _returnvalue (select `/Game/STARTHERE/Library/Enums/CoverEnum` _cover :`NewEnumerator0` _timers_disadvantage :`NewEnumerator1` _timers_open :`NewEnumerator2` _timers_light :`NewEnumerator3` _timers_medium :`NewEnumerator4` _timers_heavy :`NewEnumerator5` _timers_full :!type "Float (single-precision)"))
  (bind _returnvalue_2 (> _returnvalue 0.0))
  (bind _returnvalue_3 (`KismetSystemLibrary.K2_SetTimerDelegate` (delegate `Shoot`) (/ _returnvalue (`KismetMathLibrary.SelectFloat` 5.0 0.1 _returnvalue_2))))
  (bind _returnvalue_4 (`KismetSystemLibrary.K2_SetTimerDelegate` (delegate `ProjectileFX`) (/ _returnvalue (`KismetMathLibrary.SelectFloat` 25.0 0.1 _returnvalue_2)) true)))

(event `ProjectileFX`
  ;[1 1 1] Combat
  (`self.FireTracer`))

(event `Shoot`
  (bind _currenttarget (`self.CurrentTarget`))
  ;[1 1 1] Combat
  (`/Engine/EditorBlueprintResources/StandardMacros.IsValid` _currenttarget
    (:`Is Valid`
      (`GameplayStatics.ApplyDamage` _currenttarget 1.0)
      (set `self.ShotInt` 0)
      (`KismetSystemLibrary.K2_ClearAndInvalidateTimerHandle` (stale `/Game/STARTHERE/Library/Interfaces/CombatInterface.BeginCombat` _returnvalue_4))
      (goto _label))))

(event `EnemyDead`
  ;[1 1 1] Combat
  (set `self.CurrentTarget` null)
  (`KismetSystemLibrary.K2_ClearAndInvalidateTimerHandle` (stale `/Game/STARTHERE/Library/Interfaces/CombatInterface.BeginCombat` _returnvalue_3))
  (`KismetSystemLibrary.K2_ClearAndInvalidateTimerHandle` (stale `/Game/STARTHERE/Library/Interfaces/CombatInterface.BeginCombat` _returnvalue_4)))

(event `/Game/STARTHERE/Library/Interfaces/CombatInterface.ChangeCoverType`
  (params (Type :type "/Game/STARTHERE/Library/Enums/CoverEnum Enum" :default "NewEnumerator0"))
  (set `self.CoverType` Type))

(event `/Game/STARTHERE/Library/Interfaces/GMInterface.SetTimeZone`
  (params (`InPast?` :type Boolean))
  (set `self.Past?` `InPast?`))

(fn `CanDestroyCover`
  (returns (`True?` :type Boolean))
  (return false))

(fn `CheckCover`
  (returns (Cover :type "/Game/STARTHERE/Library/Enums/CoverEnum Enum"))
  (return (`self.CoverType`)))

(fn `FireTracer`
  (bind _returnvalue (`SceneComponent.K2_GetComponentLocation` (`self.GunPointer`)))
  (bind _returnvalue_2 (select `int` (`self.ShotInt`) :`0` 5.0 :`1` 4.0 :`2` 3.0 :`3` 2.0 :`4` 1.0))
  (bind _currenttarget (`self.CurrentTarget`)
    (:`then`
      (bind (_returnvalue_roll _returnvalue_pitch _returnvalue_yaw) (`KismetMathLibrary.BreakRotator` (`KismetMathLibrary.FindLookAtRotation` _returnvalue (`SceneComponent.K2_GetComponentLocation` (`Actor.RootComponent` _currenttarget)))))
      (`|SpawnActorFromClass` "/Game/STARTHERE/FX/Projectiles/PlayerProjectile.PlayerProjectile_C" (`KismetMathLibrary.MakeTransform` _returnvalue (`KismetMathLibrary.MakeRotator` _returnvalue_roll (`KismetMathLibrary.RandomFloatInRange` (- _returnvalue_pitch _returnvalue_2) (+ _returnvalue_pitch _returnvalue_2)) (`KismetMathLibrary.RandomFloatInRange` (- _returnvalue_yaw _returnvalue_2) (+ _returnvalue_yaw _returnvalue_2)))) "Undefined" "OverrideRootScale" null null)
      (bind _result (`/Engine/EditorBlueprintResources/StandardMacros.IncrementInt` (`self.ShotInt`))
        (:`  `
          (bind _output_get (set `self.ShotInt` _result))
          (if (> _output_get 4)
            (set `self.ShotInt` 0)))))
    (:`else`)))

(fn `GetEnemyIndex`
  (returns (Index :type Integer))
  (return 0))

(fn `GetPlayerIndex`
  (returns (PlayerIndex :type Integer))
  (return 0))

(fn `GetPlayers`
  (returns (Actors :type "Array of Actor Object Reference") (Success :type Boolean))
  (return _ false))

(fn `GetTargetLoc`
  (returns (Loc :type "Vector Structure"))
  (return (0.0 0.0 0.0)))

(fn `GetTimeZone`
  (returns (`Past?` :type Boolean))
  (return (`self.Past?`)))

(fn `Identify`
  (returns (Idenity :type "/Game/STARTHERE/Library/Enums/IdentifyEnum Enum") (Ref :type "Actor Object Reference"))
  (return (`self.Identity`) self))

(fn `InPast?`
  (returns (`Past?` :type Boolean))
  (return false))

(fn `PauseEnemies`
  (params (Pause :type Boolean) (UnPauseData :type "/Game/STARTHERE/Library/Structs/PauseEnemy Structure"))
  (returns (PauseData :type "/Game/STARTHERE/Library/Structs/PauseEnemy Structure"))
  (return))

(fn `PauseGame`
  (params (Pause :type Boolean) (UnPauseData :type "/Game/STARTHERE/Library/Structs/PauseGame Structure"))
  (returns (PauseData :type "/Game/STARTHERE/Library/Structs/PauseGame Structure"))
  (return))

(fn `PausePlayers`
  (params (Pause :type Boolean) (UnPauseData :type "/Game/STARTHERE/Library/Structs/PausePlayer Structure"))
  (returns (Pausedata :type "/Game/STARTHERE/Library/Structs/PausePlayer Structure"))
  (return))

(fn `PlayerHealth`
  (params (Index :type Integer))
  (returns (HP :type "Float (double-precision)") (Success :type Boolean))
  (return (`self.HP`) (== Index (`self.Index`))))

(fn `UserConstructionScript`)