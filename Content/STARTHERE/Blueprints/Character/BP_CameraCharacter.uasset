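; BP_CameraCharacter is a Character, apparently a camera avatar, that moves on input and tracks whether it is in the past.
; Forward and right input feed movement vectors along the capsule's axes into CharacterMovement.
; SetTimeZone sets the InPast flag and TimeTravel toggles it, with no other effect here.
; Identify returns its identity and self, while the cover, state, player and target queries return fixed placeholder values.
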(event `/Game/STARTHERE/Library/Interfaces/InputInterface.UpInput`
  (params (Alpha :type "Float (double-precision)"))
  ;[1 1 1] Read Input & Move
  (`PawnMovementComponent.AddInputVector` (`self.CharacterMovement`) (* (`SceneComponent.GetForwardVector` (`self.CapsuleComponent`)) Alpha) false))

(event `/Game/STARTHERE/Library/Interfaces/InputInterface.RightInput`
  (params (Alpha :type "Float (double-precision)"))
  ;[1 1 1] Read Input & Move
  (`PawnMovementComponent.AddInputVector` (`self.CharacterMovement`) (* (`SceneComponent.GetRightVector` (`self.CapsuleComponent`)) Alpha) false))

(event `/Game/STARTHERE/Library/Interfaces/GMInterface.SetTimeZone`
  (params (`InPast?` :type Boolean))
  (set `self.InPast` `InPast?`))

(event `/Game/STARTHERE/Library/Interfaces/InputInterface.TimeTravel`
  (params (Index :type Integer))
  (set `self.InPast` (not (`self.InPast`))))

(fn `CanDestroyCover`
  (returns (`True?` :type Boolean))
  (return false))

(fn `CheckCover`
  (returns (Cover :type "/Game/STARTHERE/Library/Enums/CoverEnum Enum"))
  (return "NewEnumerator0"))

(fn `CheckState`
  (returns (State :type "/Game/STARTHERE/Library/Enums/PlayerStates Enum"))
  (return "NewEnumerator0"))

(fn `GetPlayers`
  (returns (Actors :type "Array of Actor Object Reference") (Success :type Boolean))
  (return _ false))

(fn `GetTargetLoc`
  (returns (Loc :type "Vector Structure"))
  (return (0.0 0.0 0.0)))

(fn `Identify`
  (returns (Idenity :type "/Game/STARTHERE/Library/Enums/IdentifyEnum Enum") (Ref :type "Actor Object Reference"))
  (return (`self.Identity`) self))

(fn `InPast?`
  (returns (`Past?` :type Boolean))
  (return (`self.InPast`)))

(fn `UserConstructionScript`)