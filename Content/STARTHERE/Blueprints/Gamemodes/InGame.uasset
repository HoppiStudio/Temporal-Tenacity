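; In-game game mode that spawns the four player characters and keeps the elapsed match time.
; On BeginPlay it spawns each player class at a random point around player character 0, stores it and sends its AI controller the array index as player ID.
; A looping one-second timer advances an hour/minute/second value, though minutes never wrap.
; Getters expose players and time, while CheckState and DownInput are stubs.
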(event `self.ReceiveBeginPlay`
  (`self.Init`))

(event `Init`
  (`self.SpawnPlayers`)
  (`self.Start game timer`))

(event `SpawnPlayers`
  (for _index (range 4)
    (bind _returnvalue (`|SpawnActorFromClass` (`|GetArrayItem` (`self.PlayerClasses`) _index) (`KismetMathLibrary.MakeTransform` (`KismetMathLibrary.RandomPointInBoundingBox` (`self.K2_GetActorLocation` (`GameplayStatics.GetPlayerCharacter` 0)) (500.0 500.0 0.0))) "Undefined" "OverrideRootScale" null null))
    (bind _returnvalue_2 (`KismetArrayLibrary.Array_Add` (`self.Characters`) _returnvalue))
    (message `/Game/STARTHERE/Library/Interfaces/GMInterface.AssignPlayerID` (`AIBlueprintHelperLibrary.GetAIController` _returnvalue) _returnvalue_2)))

(event `Start game timer`
  (`KismetSystemLibrary.K2_SetTimerDelegate` (delegate `GameTimer`) 1.0 true))

(event `GameTimer`
  (bind (_timer_second _timer_minute _timer_hour) (break `/Game/STARTHERE/Library/Structs/GameTimer` (`self.Timer`)))
  (bind _returnvalue (+ _timer_second 1))
  (bind _returnvalue_2 (+ _timer_minute 1))
  (bind _returnvalue_3 (>= _returnvalue 60))
  (set `self.Timer` (make `/Game/STARTHERE/Library/Structs/GameTimer` (`KismetMathLibrary.SelectInt` 0 _returnvalue _returnvalue_3) (`KismetMathLibrary.SelectInt` _returnvalue_2 _timer_minute _returnvalue_3) (`KismetMathLibrary.SelectInt` (+ _timer_hour 1) _timer_hour (>= _returnvalue_2 60)))))

(fn `CheckState`
  (returns (State :type "/Game/STARTHERE/Library/Enums/PlayerStates Enum"))
  (return "NewEnumerator0"))

(fn `DownInput`
  (params (A :type "Float (double-precision)"))
  (return))

(fn `GetPlayers`
  (returns (Actors :type "Array of Actor Object Reference") (Success :type Boolean))
  (return (`self.Characters`) true))

(fn `GetTime`
  (returns (Time :type "/Game/STARTHERE/Library/Structs/GameTimer Structure"))
  (return (`self.Timer`)))

(fn `UserConstructionScript`)