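; Base enemy AI controller that runs a behavior tree and drives detection through neutral, alert and combat states.
; A looping sight timer traces to nearby living characters, targeting the closest visible one and reporting single-cover cases to TemporalTelemetryManager.
; After an awareness delay, a line-of-sight check starts combat, mirroring state to Blackboard and pawn.
; Combat resets on lost sight, target death or excessive distance.
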(event `self.ReceiveBeginPlay`
  (`self.Init`))

(event `Init`
  (`self.RunBehaviorTree` (`self.BT`))
  (`self.Initialise vision`)
  (bind _outactors (`GameplayStatics.GetAllActorsOfClass` "/Game/STARTHERE/Blueprints/Gamemodes/GameRules/TemporalTelemetryManager.TemporalTelemetryManager_C"))
  (for _array_element _outactors
    (set `self.TT` _array_element)))

(event `Initialise vision`
  (`KismetSystemLibrary.K2_SetTimerDelegate` (delegate `SightTick`) 1.0 true))

(event `SightTick`
  (bind _target (`self.Target`))
  ;[1 1 1] EnemySight
  (if (`self.InCombat`)
    (`/Engine/EditorBlueprintResources/StandardMacros.IsValid` _target
      (:`Is Valid`
        (if (not (<= (`self.GetDistanceTo` _target) (`self.MaxEngagementDistance`)))
          (`self.RetunToNeutral` :!label _label)))
      (:`Is Not Valid`
        (goto _label)))
    (else
      (bind _outactors (`GameplayStatics.GetAllActorsOfClass` "/Game/STARTHERE/Blueprints/Character/BP_BaseCharacter.BP_BaseCharacter_C"))
      (for _array_element _outactors
        (`self.EnemySight` _array_element))
      (set `self.NearestPlayerDist` 0.0)
      (if (not (and (`self.Alert`) (`self.InCombat`)))
        (`/Engine/EditorBlueprintResources/StandardMacros.IsValid` (`self.Target`)
          (:`Is Valid`
            (set `self.Alert` true)
            (`self.SetState` 1)
            (`KismetSystemLibrary.Delay` (`self.Awareness`))
            (`self.LineOfSightTest`
              (:`Success`
                (set `self.InCombat` true)
                (set `self.Alert` true)
                (`self.SetState` 2)
                (`self.StartCombat`))
              (:`Fail`
                (set `self.InCombat` false)
                (set `self.Alert` false)
                (`self.SetState` 0))))
          (:`Is Not Valid`
            (set `self.Target` null)))))))

(event `StartCombat`
  (bind _target (`self.Target`))
  ;[1 1 1] Combat
  (`/Engine/EditorBlueprintResources/StandardMacros.IsValid` _target
    (:`Is Valid`
      (bind _asbp_base_character (cast `/Game/STARTHERE/Blueprints/Character/BP_BaseCharacter` _target))
      (if (`/Game/STARTHERE/Blueprints/Character/BP_BaseCharacter.Dead` _asbp_base_character)
        (`self.StopCombat` 0 :!label _label_2)
        (`self.Test`)
        (else
          (add `/Game/STARTHERE/Blueprints/Character/BP_BaseCharacter.PlayerDead` _asbp_base_character (delegate `StopCombat`))
          (add `/Game/STARTHERE/Blueprints/Character/BP_BaseCharacter.Test` _asbp_base_character (delegate `Test`))
          (message `/Game/STARTHERE/Library/Interfaces/CombatInterface.BeginCombat` (`self.K2_GetPawn`) _target)
          (`KismetSystemLibrary.K2_SetTimerDelegate` (delegate `CombatLOS`) 0.5 true))))
    (:`Is Not Valid`
      (goto _label_2))))

(event `CombatLOS`
  ;[1 1 1] Combat
  (`self.LineOfSightTest`
    (:`Success`
      (bind _dead (message `/Game/STARTHERE/Library/Interfaces/CombatInterface.Isdead` (`self.Target`)))
      (if _dead
        (`self.StopCombat` 0 :!label _label_3)
        (`self.Test`)))
    (:`Fail`
      (goto _label_3))))

(event `Test`
  (bind _target (`self.Target`))
  ;[1 1 1] Combat
  (`/Engine/EditorBlueprintResources/StandardMacros.IsValid` _target
    (:`Is Valid`
      (bind _asbp_base_character (cast `/Game/STARTHERE/Blueprints/Character/BP_BaseCharacter` _target)
        (:`then`
          (clear `/Game/STARTHERE/Blueprints/Character/BP_BaseCharacter.PlayerDead` _asbp_base_character)
          (clear `/Game/STARTHERE/Blueprints/Character/BP_BaseCharacter.Test` _asbp_base_character))
        (:`CastFailed`
          _)))
    (:`Is Not Valid`
      _))
  (`self.RetunToNeutral`)
  (message `/Game/STARTHERE/Library/Interfaces/CombatInterface.EndCombat` (`self.K2_GetPawn`)))

(event `StopCombat`
  (params (Index :type Integer))
  ;[1 1 1] Combat
)

(fn `EnemySight`
  (params (Ref :type "/Game/STARTHERE/Blueprints/Character/BP_BaseCharacter Object Reference"))
  (returns (Targeted :type Boolean) (TTcoverAlert :type Boolean))
  (locals (CoverRef :type "/Game/STARTHERE/Blueprints/GameObjects/Cover/BP_BaseCover Object Reference") (TargetSet :type Boolean) (SingleCover :type Boolean) (Cover :type Boolean) (PlayerRef :type "/Game/STARTHERE/Blueprints/Character/BP_BaseCharacter Object Reference"))
  (bind _returnvalue (`self.K2_GetPawn`))
  (bind (_returnvalue_x _returnvalue_y _returnvalue_z) (`KismetMathLibrary.BreakVector` (`self.K2_GetActorLocation` Ref)))
  (bind (_returnvalue_x_2 _returnvalue_y_2 _returnvalue_z_2) (`KismetMathLibrary.BreakVector` (`self.K2_GetActorLocation` _returnvalue)))
  (if (`/Game/STARTHERE/Blueprints/Character/BP_BaseCharacter.Dead` Ref)
    _
    (elif (<= (`self.GetDistanceTo` _returnvalue Ref) 10000.0)
      (set `local.PlayerRef` null)
      (set `local.CoverRef` null)
      (set `local.TargetSet` false)
      (set `local.SingleCover` false)
      (set `local.Cover` false)
      (bind _outhits (`KismetSystemLibrary.LineTraceMultiForObjects` (`KismetMathLibrary.MakeVector` _returnvalue_x_2 _returnvalue_y_2 (+ _returnvalue_z_2 100.0)) (`KismetMathLibrary.MakeVector` _returnvalue_x _returnvalue_y (+ _returnvalue_z 75.0)) (`|MakeArray` "ObjectTypeQuery2" "ObjectTypeQuery1" "ObjectTypeQuery3" :!type "EObjectTypeQuery Enum") true (`|MakeArray` _returnvalue :!type "Actor Object Reference") "None" true (struct :`R` 1.0 :`A` 1.0) (struct :`G` 1.0 :`A` 1.0) 1.0))
      (for _array_element _outhits
        (bind (_bblockinghit _binitialoverlap _time _distance _location _impactpoint _normal _impactnormal _physmat _hitactor _hitcomponent) (`GameplayStatics.BreakHitResult` _array_element))
        (if (`GameplayStatics.ObjectIsA` _hitcomponent "/Script/Engine.BoxComponent")
          _
          (elif (or (`GameplayStatics.ObjectIsA` _hitactor "/Script/Engine.StaticMeshActor") (`GameplayStatics.ObjectIsA` _hitactor "/Script/Engine.StaticMesh"))
            (break)
            (elif (`GameplayStatics.ObjectIsA` _hitactor "/Game/STARTHERE/Blueprints/GameObjects/Cover/BP_BaseCover.BP_BaseCover_C")
              (bind _asbp_base_cover (cast `/Game/STARTHERE/Blueprints/GameObjects/Cover/BP_BaseCover` _hitactor))
              (`|ExecutionSequence`
                (:`then_0`
                  (if (`local.SingleCover`)
                    (set `local.SingleCover` false)
                    (set `local.Cover` true)))
                (:`then_1`
                  (`/Engine/EditorBlueprintResources/StandardMacros.DoOnce` false
                    (:`Completed`
                      (set `local.SingleCover` true)
                      (set `local.Cover` true)
                      (set `local.PlayerRef` Ref)
                      (set `local.CoverRef` _asbp_base_cover)))))
              (else
                (`self.CanSeePlayer` _distance Ref
                  (:`ChangeTarget`
                    (set `local.PlayerRef` Ref)
                    (set `local.TargetSet` true))))))))
      (if (`local.SingleCover`)
        (bind _asbp_base_enemy (cast `/Game/STARTHERE/Blueprints/Enemies/BP_BaseEnemy` (`self.K2_GetPawn`)))
        (message `/Game/STARTHERE/Library/Interfaces/TTInterface.PlayerInCover` (`self.TT`) _asbp_base_enemy (`local.PlayerRef`) (`local.CoverRef`))
        (return false true)
        (else
          (if (`local.TargetSet`)
            (if (`local.Cover`)
              _
              (else
                (set `self.Target` (`local.PlayerRef`))
                (return true false))))
          (return false false))))))

(fn `RetunToNeutral`
  (set `self.InCombat` false)
  (set `self.Alert` false)
  (`self.SetState` 0)
  (set `self.Target` null))

(fn `SetState`
  (params (Index :type Integer))
  (set `self.AIState` Index)
  (`BlackboardComponent.SetValueAsInt` (`AIBlueprintHelperLibrary.GetBlackboard` null) "StateIndex" Index)
  (message `/Game/STARTHERE/Library/Interfaces/UIInterface.EnemyInfo` (`self.K2_GetPawn`) 0.0 0.0 Index)
  (return))

(fn `UserConstructionScript`)